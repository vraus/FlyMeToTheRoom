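; BP_MugInteractionActor_Child is a child interaction actor in the TapKey system, judging by its name a configurable variant of the mug interaction actor.
; Its construction script runs the parent's, then applies the mesh and material variables to the Cube component and the radius variable to the Sphere component.
; It adds no runtime logic of its own, as its event graph holds only disabled placeholder events.
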(event EventBeginPlay
  (|CallParentFunction) ; This node is disabled and will not be called.\nDrag off pins to build functionality.
)

(event Collision|EventActorBeginOverlap
  (params (OtherActor :type Actor%20Object%20Reference)))

(event EventTick
  (params (DeltaSeconds :type Float%20%28single-precision%29)))

(fn ConstructionScript
  (|CallParentFunction)
  (Components|StaticMesh|SetStaticMesh (Variables|Default|GetCube) (Variables|Default|GetStatic%20Mesh))
  (Rendering|Material|SetMaterial (Variables|Default|GetCube) 0 (Variables|Default|GetMaterial))
  (Components|Sphere|SetSphereRadius (Variables|Default|GetSphere) (Variables|Default|GetSphereRadius) true))