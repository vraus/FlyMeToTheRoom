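; BP_SpiderWeb is a spider web hazard actor that triggers a timed tap-key prompt when the player's fly pawn (P_Fly) touches it.
; Entering the Box highlights the Cube through custom depth, starts an F-key tap event on the fly, and fades a new WB_DamageScreen widget.
; Leaving the Box clears the highlight and removes the tap event.
; The Sphere overlap events are empty.
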(event OnComponentBeginOverlap(Box)
  (params (OverlappedComponent :type Primitive%20Component%20Object%20Reference) (OtherActor :type Actor%20Object%20Reference) (OtherComp :type Primitive%20Component%20Object%20Reference) (OtherBodyIndex :type Integer) (bFromSweep :type Boolean) (SweepResult :type Hit%20Result%20Structure%20%28by%20ref%29))
  (bind _asp_fly (Utilities|Casting|CastToP_Fly OtherActor))
  (Rendering|SetRenderCustomDepth (Variables|Default|GetCube) true)
  (Default|CreateTapKeyEvent _asp_fly "F" true 0.2 "F" self)
  (bind _returnvalue (UserInterface|CreateWidget "/Game/DTJ/Blueprints/UI/WB_DamageScreen.WB_DamageScreen_C"))
  (UserInterface|Viewport|AddtoViewport _returnvalue 0)
  (Default|PlayFade _returnvalue))

(event OnComponentEndOverlap(Box)
  (params (OverlappedComponent :type Primitive%20Component%20Object%20Reference) (OtherActor :type Actor%20Object%20Reference) (OtherComp :type Primitive%20Component%20Object%20Reference) (OtherBodyIndex :type Integer))
  (bind _asp_fly (Utilities|Casting|CastToP_Fly OtherActor))
  (Rendering|SetRenderCustomDepth (Variables|Default|GetCube) false)
  (Default|RemoveTapKeyEvent _asp_fly))

(event OnComponentBeginOverlap(Sphere)
  (params (OverlappedComponent :type Primitive%20Component%20Object%20Reference) (OtherActor :type Actor%20Object%20Reference) (OtherComp :type Primitive%20Component%20Object%20Reference) (OtherBodyIndex :type Integer) (bFromSweep :type Boolean) (SweepResult :type Hit%20Result%20Structure%20%28by%20ref%29)))

(event OnComponentEndOverlap(Sphere)
  (params (OverlappedComponent :type Primitive%20Component%20Object%20Reference) (OtherActor :type Actor%20Object%20Reference) (OtherComp :type Primitive%20Component%20Object%20Reference) (OtherBodyIndex :type Integer)))

(event EventBeginPlay
  (|CallParentFunction) ; This node is disabled and will not be called.\nDrag off pins to build functionality.
)

(event Collision|EventActorBeginOverlap
  (params (OtherActor :type Actor%20Object%20Reference))
  (|CallParentFunction OtherActor) ; This node is disabled and will not be called.\nDrag off pins to build functionality.
)

(event EventTick
  (params (DeltaSeconds :type Float%20%28single-precision%29))
  (|CallParentFunction DeltaSeconds) ; This node is disabled and will not be called.\nDrag off pins to build functionality.
)

(fn ConstructionScript
  (|CallParentFunction))