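; An interaction actor whose cube starts physics simulation, letting it fall, through the tap-key system of the P_Fly pawn.
; Entering the sphere enables the cube's custom depth and registers a G key prompt on the pawn; leaving reverses both.
; PressedFonctionality enables physics and removes the prompt, reusing the pawn reference from the end-overlap cast, which is unset until an overlap has ended.
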(event OnComponentBeginOverlap(Sphere)
  (params (OverlappedComponent :type Primitive%20Component%20Object%20Reference) (OtherActor :type Actor%20Object%20Reference) (OtherComp :type Primitive%20Component%20Object%20Reference) (OtherBodyIndex :type Integer) (bFromSweep :type Boolean) (SweepResult :type Hit%20Result%20Structure%20%28by%20ref%29))
  (bind _asp_fly (Utilities|Casting|CastToP_Fly OtherActor))
  (Rendering|SetRenderCustomDepth (Variables|Default|GetCube) true)
  (Default|CreateTapKeyEvent _asp_fly "G" false 0.0 "G" self))

(event OnComponentEndOverlap(Sphere)
  (params (OverlappedComponent :type Primitive%20Component%20Object%20Reference) (OtherActor :type Actor%20Object%20Reference) (OtherComp :type Primitive%20Component%20Object%20Reference) (OtherBodyIndex :type Integer))
  (bind _asp_fly (Utilities|Casting|CastToP_Fly OtherActor))
  (Rendering|SetRenderCustomDepth (Variables|Default|GetCube) false)
  (Default|RemoveTapKeyEvent _asp_fly))

(event EventPressedFonctionality
  (params (Direction :type Vector :default "0, 0, 0"))
  (Physics|SetSimulatePhysics (Variables|Default|GetCube) true)
  (Default|RemoveTapKeyEvent (stale OnComponentEndOverlap(Sphere) _asp_fly)))

(fn ConstructionScript)