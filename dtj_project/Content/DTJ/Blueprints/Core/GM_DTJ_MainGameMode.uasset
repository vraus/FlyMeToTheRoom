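; Main game mode that tracks how many flies the player saves and triggers the win or loss screen.
; On begin play it counts the BP_DangerInteractionActor_Child actors as the fly total and shows a counter widget.
; Each TapKeySuccess event raises the saved count, updates the counter and triggers the win once all are saved.
; GMLoose triggers defeat; both outcomes show a screen, the mouse cursor and play a sound.
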(event Custom|WIn
  (bind _returnvalue (UserInterface|CreateWidget "/Game/DTJ/Blueprints/UI/WB_WinScreen.WB_WinScreen_C"))
  (UserInterface|Viewport|AddtoViewport _returnvalue 0)
  (Variables|/Script/Engine.PlayerController|SetbShowMouseCursor (Game|GetPlayerController 0) true)
  (Audio|PlaySound2D "/Game/DTJ/SFX/VictorySound.VictorySound" 1.0 1.0 0.0 0 0))

(event Custom|Loose
  (bind _returnvalue (UserInterface|CreateWidget "/Game/DTJ/Blueprints/UI/WB_Loose.WB_Loose_C"))
  (UserInterface|Viewport|AddtoViewport _returnvalue 0)
  (Variables|/Script/Engine.PlayerController|SetbShowMouseCursor (Game|GetPlayerController 0) true)
  (Audio|PlaySound2D "/Game/DTJ/SFX/DefeatSound.DefeatSound" 1.0 1.0 0.0 0 0))

(event EventBeginPlay
  (bind _outactors (Actor|GetAllActorsOfClass "/Game/DTJ/Blueprints/TapKeySystem/BP_DangerInteractionActor_Child.BP_DangerInteractionActor_Child_C"))
  (Variables|Default|SetMaxFlies (Utilities|Array|Length _outactors))
  (bind _returnvalue (UserInterface|CreateWidget "/Game/DTJ/Blueprints/UI/WBC_FlyCount.WBC_FlyCount_C" 0 0 (Variables|Default|GetMaxFlies)))
  (bind _output_get (Variables|Default|SetFlyCount _returnvalue))
  (UserInterface|Viewport|AddtoViewport _output_get 0))

(event EventTapKeySuccess
  (Math|Integer|IncrementInt (Variables|Default|GetSavedFlyCount)
    (:%20%20
      (CallFunction|CheckWinConditions)
      (Default|UpdateFlyCount (Variables|Default|GetFlyCount) (Variables|Default|GetSavedFlyCount) (Variables|Default|GetMaxFlies)))))

(event EventGMLoose
  (CallFunction|Loose))

(fn ConstructionScript)

(fn CheckWinConditions
  (if (== (Variables|Default|GetSavedFlyCount) (Variables|Default|GetMaxFlies))
    (CallFunction|Win)))