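; Player controller for the fly game that sets up Enhanced Input for the player's keyboard layout.
; On BeginPlay it reads the AZERTY flag from GI_FlyMeToTheRoom and adds either the IMC_Fly or IMC_Fly_Qwerty mapping context.
; A debug key on H calls the win function on GM_DTJ_MainGameMode as a shortcut to victory.
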(event EventBeginPlay
  (bind _returnvalue (PlayerController|LocalPlayerSubsystems|GetEnhancedInputLocalPlayerSubsystem))
  (Utilities|IsValid _returnvalue
    (:Is%20Valid
      (if (Variables|/Game/DTJ/Blueprints/Core/GI_FlyMeToTheRoom.GI_FlyMeToTheRoom_C|GetbIsInAZERTY (.AsGI%20Fly%20Me%20to%20the%20Room (Utilities|Casting|CastToGI_FlyMeToTheRoom (Game|GetGameInstance))))
        (Input|AddMappingContext _returnvalue "/Game/DTJ/Blueprints/Fly/Inputs/IMC_Fly.IMC_Fly" 0 "(bIgnoreAllPressedKeysUntilRelease=True,bForceImmediately=False,bNotifyUserSettings=False)")
        (else
          (Input|AddMappingContext _returnvalue "/Game/DTJ/Blueprints/Fly/Inputs/IMC_Fly_Qwerty.IMC_Fly_Qwerty" 0 "(bIgnoreAllPressedKeysUntilRelease=True,bForceImmediately=False,bNotifyUserSettings=False)"))))))

(event Input|KeyboardEvents|DebugKeyH
  (params (Key :type Key%20Structure :default "None") (ActionValue :type Input%20Action%20Value%20Structure))
  (:Pressed
    (bind _asgm_dtj_main_game_mode (Utilities|Casting|CastToGM_DTJ_MainGameMode (Game|GetGameMode)))
    (Default|Win _asgm_dtj_main_game_mode)))

(fn ConstructionScript)